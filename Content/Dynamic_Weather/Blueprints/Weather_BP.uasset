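; Dynamic weather actor that drives rain, snow, lightning, fog, surface decal, sound and post-process effects from humidity and temperature.
; RefreshWeather splits humidity into rain and snow by a temperature curve, feeding particles, materials and parameter collections.
; Optional seeded, interpolated noise varies both inputs in realtime, while particles follow the player.
; An orthographic scene capture of listed actors, taken at BeginPlay, provides object detection.
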(event `self.ReceiveBeginPlay`
  (bind _random_stream (`self.Random Stream`))
  ;[1 1 1] Initialize Random Perlin Noise Start Values and Refresh Weather
  (`|ExecutionSequence`
    (:`then_0`
      (`KismetMathLibrary.SetRandomStreamSeed` _random_stream (`self.Random Seed`)))
    (:`then_1`
      (set `self.P1 Humidity` (`KismetMathLibrary.RandomFloatInRangeFromStream` (`self.Minimum Humidity`) (`self.Maximum Humidity`) _random_stream)))
    (:`then_2`
      (set `self.P1 Temperature` (`KismetMathLibrary.RandomFloatInRangeFromStream` (`self.Minimum Temperature`) (`self.Maximum Temperature`) _random_stream)))
    (:`then_3`
      (`self.Refresh Weather`)
      (`self.Object Detection`)
      (`SceneCaptureComponent2D.CaptureScene` (`self.Detect_Below`)))))

(event `self.ReceiveTick`
  (params (DeltaSeconds :type "Float (single-precision)"))
  (bind _rain_emitter (`self.Rain_Emitter`))
  (bind _realtime_random_humidity (`self.Realtime Random Humidity`))
  (bind _realtime_random_temperature (`self.Realtime Random Temperature`))
  ;[1 1 1] Realtime Random Weather
  (`|ExecutionSequence`
    (:`then_0`
      (if _realtime_random_humidity
        (`self.Randomize Humidity` (`self.Random Humidity Time`))))
    (:`then_1`
      (if (or _realtime_random_humidity _realtime_random_temperature)
        (`self.Refresh Weather`)))
    (:`then_2`
      (if _realtime_random_temperature
        (`self.Randomize Temperature` (`self.Random Temperature Time`))))
    (:`then_3`
      ;[1 1 1] Particles Follow Player
      (if (`self.Use Rain / Snow`)
        (`/Engine/EditorBlueprintResources/StandardMacros.IsValid` (`self.Snow_Emitter`)
          (:`Is Valid`
            (`/Engine/EditorBlueprintResources/StandardMacros.IsValid` _rain_emitter
              (:`Is Valid`
                (`SceneComponent.K2_SetWorldLocation` _rain_emitter (`self.K2_GetActorLocation` (`Controller.K2_GetPawn` (`GameplayStatics.GetPlayerController` 0))) false false)
                (`SceneComponent.K2_SetWorldLocation` (`self.Snow_Emitter`) (`self.K2_GetActorLocation` (`Controller.K2_GetPawn` (`GameplayStatics.GetPlayerController` 0))) false false)))))))))

(fn `Humidity Perlin Noise`
  (params (`Change Speed` :type "Float (double-precision)"))
  (returns (ReturnValue :type "Float (double-precision)"))
  (bind _returnvalue (`GameplayStatics.GetTimeSeconds`))
  (bind _position_humidity (`self.Position Humidity`))
  (bind _p0_humidity (`self.P0 Humidity`))
  (bind _timer_humidity (`self.Timer Humidity`))
  (if (> _returnvalue _timer_humidity)
    (set `self.Timer Humidity` (+ _timer_humidity `Change Speed`))
    (set `self.P0 Humidity` (`self.P1 Humidity`))
    (set `self.P1 Humidity` (`KismetMathLibrary.RandomFloatInRangeFromStream` 0.0 1.0 (`self.Random Stream`)))
    (return (`self.P0 Humidity`))
    (else
      (set `self.Position Humidity` (/ (- `Change Speed` (- _timer_humidity _returnvalue)) `Change Speed`))
      (return (+ (* (+ (* (`KismetMathLibrary.MultiplyMultiply_FloatFloat` _position_humidity 3.0) -1.0) (* (`KismetMathLibrary.MultiplyMultiply_FloatFloat` _position_humidity 2.0) 2.0)) (- (`self.P1 Humidity`) _p0_humidity)) _p0_humidity)))))

(fn `Object Detection`
  (bind (_returnvalue_x _returnvalue_y) (`KismetMathLibrary.BreakVector` (`self.K2_GetActorLocation`)))
  (bind _detect_below (`self.Detect_Below`))
  (`KismetMaterialLibrary.SetVectorParameterValue` "/Game/Dynamic_Weather/Materials/Capture_Collection.Capture_Collection" "Location" (`KismetMathLibrary.Conv_VectorToLinearColor` (`KismetMathLibrary.MakeVector` _returnvalue_x _returnvalue_y)))
  (`KismetMaterialLibrary.SetScalarParameterValue` "/Game/Dynamic_Weather/Materials/Capture_Collection.Capture_Collection" "Bounds" (`self.Scene Capture Size`))
  (`KismetMaterialLibrary.SetScalarParameterValue` "/Game/Dynamic_Weather/Materials/Capture_Collection.Capture_Collection" "Height" (`self.Scene Capture Height`))
  (set `SceneCaptureComponent2D.OrthoWidth` (`self.Scene Capture Size`) _detect_below)
  (`SceneComponent.K2_SetWorldLocation` _detect_below (`KismetMathLibrary.MakeVector` _returnvalue_x _returnvalue_y (`self.Scene Capture Height`)) false false)
  (for _array_element (`self.Object Array`)
    (`SceneCaptureComponent.ShowOnlyActorComponents` _detect_below _array_element false)
    (`KismetMaterialLibrary.SetScalarParameterValue` "/Game/Dynamic_Weather/Materials/Distort_Collection.Distort_Collection" "Scale" (`self.Distortion Scale`))
    (`KismetMaterialLibrary.SetScalarParameterValue` "/Game/Dynamic_Weather/Materials/Distort_Collection.Distort_Collection" "Distortion" (`self.Distortion Intensity`))))

(fn `Randomize Humidity`
  (params (`Change Speed` :type "Float (double-precision)"))
  (bind _minimum_humidity (`self.Minimum Humidity`))
  (bind _returnvalue (`self.Humidity Perlin Noise` `Change Speed`))
  (set `self.Humidity` (+ (* _returnvalue (- (`self.Maximum Humidity`) _minimum_humidity)) _minimum_humidity)))

(fn `Randomize Temperature`
  (params (`Change Speed` :type "Float (double-precision)"))
  (bind _returnvalue (`self.Termperature Perlin Noise` `Change Speed`))
  (set `self.Temperature (Celsius)` (+ (* _returnvalue (- (`self.Maximum Temperature`) (`self.Minimum Temperature`))) (`self.Minimum Temperature`))))

(fn `Refresh Weather`
  (bind _dirtmask (`self.Dirtmask`))
  (bind _dirtmask_intensity (`self.Dirtmask Intensity`))
  (bind _decal (`self.Decal`))
  (bind _use_rain___snow (`self.Use Rain / Snow`))
  (bind _humidity (`self.Humidity`))
  (bind _fog (`self.Fog`))
  (bind _returnvalue (`CurveFloat.GetFloatValue` (`self.Temerature Curve`) (`self.Temperature (Celsius)`)))
  (bind _returnvalue_2 (`CurveFloat.GetFloatValue` (`self.Temerature Curve`) (`self.Temperature (Celsius)`)))
  (bind _settings (`PostProcessComponent.Settings` (`self.Post_Processing`)))
  (bind _returnvalue_3 (* (`self.Rain Amount`) (`KismetMathLibrary.Conv_BoolToDouble` _use_rain___snow)))
  (`|ExecutionSequence`
    (:`then_0`
      ;[1 1 1] General
      (`self.K2_SetActorRotation` (struct))
      (`SceneComponent.SetWorldScale3D` (`self.Weatherdome`) (`KismetMathLibrary.Conv_DoubleToVector` (`self.Weatherdome Scale`))))
    (:`then_1`
      ;[1 1 1] Lightning Effect
      (bind _returnvalue_4 (`PrimitiveComponent.CreateDynamicMaterialInstance` (`self.Weatherdome`) 0 "/Game/Dynamic_Weather/Materials/Lightning_mat.Lightning_mat" "None")))
    (:`then_2`
      (`MaterialInstanceDynamic.SetScalarParameterValue` _returnvalue_4 "Lightning Power" (`self.Lightning Power`))
      (`MaterialInstanceDynamic.SetVectorParameterValue` _returnvalue_4 "Color" (`KismetMathLibrary.Conv_ColorToLinearColor` (`self.Color`)))
      (`MaterialInstanceDynamic.SetScalarParameterValue` _returnvalue_4 "Lightning Enabled" (`KismetMathLibrary.Conv_BoolToDouble` (`self.Use Lightning Effects`))))
    (:`then_3`
      (`KismetMaterialLibrary.SetScalarParameterValue` "/Game/Dynamic_Weather/Materials/Lightning_Collection.Lightning_collection" "Lightning Enabled" (`KismetMathLibrary.Conv_BoolToDouble` (and (`self.Use Lightning Effects`) (`self.Lightning Postprocessing`)))))
    (:`then_4`
      ;[1 1 1] Rain and Snow Effect
      (set `self.Rain Amount` (* _humidity _returnvalue))
      (set `self.Snow Amount` (* _humidity (- 1.0 _returnvalue))))
    (:`then_5`
      (`KismetMaterialLibrary.SetScalarParameterValue` "/Game/Dynamic_Weather/Materials/Rain_Collection.Rain_collection" "Rain Enabled" (`KismetMathLibrary.Conv_BoolToDouble` (and _use_rain___snow (`self.Rain Postprocessing`))))
      (`KismetMaterialLibrary.SetScalarParameterValue` "/Game/Dynamic_Weather/Materials/Rain_Collection.Rain_collection" "Rain Amount" _returnvalue_3))
    (:`then_6`
      (`ParticleSystemComponent.SetFloatParameter` (`self.Rain_Emitter`) "Rain Amount" _returnvalue_3))
    (:`then_7`
      (`KismetMaterialLibrary.SetScalarParameterValue` "/Game/Dynamic_Weather/Materials/Frost_Collection.Frost_collection" "Frost Enabled" (`KismetMathLibrary.Conv_BoolToDouble` (and (`self.Use Rain / Snow`) (`self.Snow Postprocessing`))))
      (`KismetMaterialLibrary.SetScalarParameterValue` "/Game/Dynamic_Weather/Materials/Frost_Collection.Frost_collection" "Frost Amount" (`self.Snow Amount`)))
    (:`then_8`
      (`ParticleSystemComponent.SetFloatParameter` (`self.Snow_Emitter`) "Snow Amount" (* (`self.Snow Amount`) (`KismetMathLibrary.Conv_BoolToDouble` _use_rain___snow))))
    (:`then_9`
      (`DecalComponent.SetDecalMaterial` _decal "/Game/Dynamic_Weather/Materials/Surface_Decal_inst.Surface_Decal_inst")
      (bind _returnvalue_5 (`DecalComponent.CreateDynamicMaterialInstance` _decal))
      (`MaterialInstanceDynamic.SetScalarParameterValue` _returnvalue_5 "Temperature" (`CurveFloat.GetFloatValue` (`self.Temerature Curve`) (`self.Temperature (Celsius)`)))
      (`MaterialInstanceDynamic.SetScalarParameterValue` _returnvalue_5 "Humidity" (`self.Humidity`))
      (`MaterialInstanceDynamic.SetScalarParameterValue` _returnvalue_5 "Scale" (`self.Decal Scale`))
      (`MaterialInstanceDynamic.SetTextureParameterValue` _returnvalue_5 "Rain Texture" (`self.Rain Texture`))
      (`MaterialInstanceDynamic.SetTextureParameterValue` _returnvalue_5 "Snow Texture" (`self.Snow Texture`)))
    (:`then_10`
      (`SceneComponent.SetVisibility` _decal (and (`self.Enable Decal`) (`self.Use Rain / Snow`)) false)
      (`SceneComponent.SetWorldScale3D` (`self.Decal`) (`KismetMathLibrary.Conv_DoubleToVector` (`self.Decal Area (World Coverage)`))))
    (:`then_11`
      (`AudioComponent.SetVolumeMultiplier` (`self.Rain_cue`) (* (* _returnvalue_2 (`self.Humidity`)) (`self.Sound Volume`)))
      (`AudioComponent.SetVolumeMultiplier` (`self.Wind_cue`) (* (* (- 1.0 _returnvalue_2) (`self.Humidity`)) (`self.Sound Volume`))))
    (:`then_12`
      (`SceneComponent.SetVisibility` (`self.Rain_Emitter`) (`self.Enable Particles`) false)
      (`SceneComponent.SetVisibility` (`self.Snow_Emitter`) (`self.Enable Particles`) false))
    (:`then_13`
      ;[1 1 1] Postprocess Effects
      (if (`self.Use Color Postprocessing`)
        (setmembers `PostProcessSettings` :`StructRef` _settings :`WhiteTemp` (`CurveFloat.GetFloatValue` (`self.Heat Curve`) (`self.Temperature (Celsius)`)) :`BloomDirtMask` _dirtmask :`BloomDirtMaskIntensity` _dirtmask_intensity)
        (else
          (setmembers `PostProcessSettings` :`StructRef` _settings :`WhiteTemp` 6500.0 :`BloomDirtMask` _dirtmask :`BloomDirtMaskIntensity` _dirtmask_intensity))))
    (:`then_14`
      ;[1 1 1] Fog Settings
      (`ExponentialHeightFogComponent.SetFogDensity` _fog (* (`self.Humidity`) (`self.Fog Density`)))
      (`ExponentialHeightFogComponent.SetFogHeightFalloff` _fog (`self.Fog Falloff`)))
    (:`then_15`
      (`SceneComponent.SetVisibility` _fog (`self.Use Height Fog`) false)
      (`ExponentialHeightFogComponent.SetVolumetricFog` _fog (`self.Volumetric Fog`))
      (`ExponentialHeightFogComponent.SetVolumetricFogExtinctionScale` _fog (`self.Volumetric Fog Density`))
      (`ExponentialHeightFogComponent.SetVolumetricFogScatteringDistribution` _fog (`self.Volumetric Fog Scattering`)))))

(fn `Termperature Perlin Noise`
  (params (`Change Speed` :type "Float (double-precision)"))
  (returns (ReturnValue :type "Float (double-precision)"))
  (bind _returnvalue (`GameplayStatics.GetTimeSeconds`))
  (bind _timer_temperature (`self.Timer Temperature`))
  (bind _p0_temperature (`self.P0 Temperature`))
  (bind _position_temperature (`self.Position Temperature`))
  (if (> _returnvalue _timer_temperature)
    (set `self.Timer Temperature` (+ _timer_temperature `Change Speed`))
    (set `self.P0 Temperature` (`self.P1 Temperature`))
    (set `self.P1 Temperature` (`KismetMathLibrary.RandomFloatInRangeFromStream` 0.0 1.0 (`self.Random Stream`)))
    (return (`self.P0 Temperature`))
    (else
      (set `self.Position Temperature` (/ (- `Change Speed` (- _timer_temperature _returnvalue)) `Change Speed`))
      (return (+ (* (+ (* (`KismetMathLibrary.MultiplyMultiply_FloatFloat` _position_temperature 3.0) -1.0) (* (`KismetMathLibrary.MultiplyMultiply_FloatFloat` _position_temperature 2.0) 2.0)) (- (`self.P1 Temperature`) _p0_temperature)) _p0_temperature)))))

(fn `UserConstructionScript`
  (`self.Refresh Weather`)
  (`self.Object Detection`))