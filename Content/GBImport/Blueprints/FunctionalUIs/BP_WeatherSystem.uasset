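; Weather controller that exposes events to change cloud density, fog, rain and snow in the level.
; The construction script caches the first Ultra Dynamic Sky, Weather_BP, SkyLight and height fog actors, though SkyLight is unused here.
; Timelines blend cloud and fog density from their last stored values to new targets.
; Rain (marked unfinished) and snow instantly set Weather_BP temperature and humidity; cloud changes also reset temperature to the rain value.
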(event `CE_ChangeCloudDensity`
  (params (newCloudDensity :type "Float (double-precision)"))
  (bind _ultra_dynamic_sky_sphere (`self.ultra_dynamic_sky_sphere`))
  (bind _lastclouddensity (`self.lastCloudDensity`))
  (bind _returnvalue (- newCloudDensity _lastclouddensity))
  ;[1 1 1] 调节云的密度、
  (set `/Game/Dynamic_Weather/Blueprints/Weather_BP.Temperature (Celsius)` 8.0 (`self.BP_Weather`))
  (bind (_direction _clouddensity) (`Timeline|1` :!via `PlayFromStart`)
    (:`Update`
      (if (> _returnvalue 0.0)
        (bind _returnvalue_2 (* _clouddensity (`KismetMathLibrary.Abs` _returnvalue)))
        (set `/Game/UltraDynamicSky/Blueprints/Ultra_Dynamic_Sky_BP.Cloud Density` (+ _lastclouddensity _returnvalue_2) _ultra_dynamic_sky_sphere)
        (else
          (set `/Game/UltraDynamicSky/Blueprints/Ultra_Dynamic_Sky_BP.Cloud Density` (- _lastclouddensity _returnvalue_2) _ultra_dynamic_sky_sphere))))
    (:`Finished`
      (set `self.lastCloudDensity` newCloudDensity))))

(event `CE_SetFogAndHaze`
  (params (newFogDensity :type "Float (double-precision)"))
  (bind _lastfogdensity (`self.lastFogDensity`))
  (bind _returnvalue (- newFogDensity _lastfogdensity))
  (bind _component (`ExponentialHeightFog.Component` (`self.EXP_fog`)))
  ;[1 1 1] 调节雾的浓度
  (bind (_direction _clouddensity) (`Timeline|2` :!via `PlayFromStart`)
    (:`Update`
      (if (> _returnvalue 0.0)
        (bind _returnvalue_2 (* _clouddensity (`KismetMathLibrary.Abs` _returnvalue)))
        (`ExponentialHeightFogComponent.SetFogDensity` _component (+ _lastfogdensity _returnvalue_2))
        (else
          (`ExponentialHeightFogComponent.SetFogDensity` _component (- _lastfogdensity _returnvalue_2)))))
    (:`Finished`
      (set `self.lastFogDensity` newFogDensity))))

(event `CE_SetRainDensity`
  (params (newRainDensity :type "Float (double-precision)"))
  (bind _bp_weather (`self.BP_Weather`))
  ;[1 1 1] 调节雨的开关和大小 (未完成)
  (set `/Game/Dynamic_Weather/Blueprints/Weather_BP.Temperature (Celsius)` 8.0 _bp_weather)
  (set `/Game/Dynamic_Weather/Blueprints/Weather_BP.Humidity` newRainDensity _bp_weather))

(event `CE_SetSnowDensity`
  (params (newSnowDensity :type "Float (double-precision)"))
  (bind _bp_weather (`self.BP_Weather`))
  ;[1 1 1] 调节雪的大小
  (set `/Game/Dynamic_Weather/Blueprints/Weather_BP.Temperature (Celsius)` -10.0 _bp_weather)
  (set `/Game/Dynamic_Weather/Blueprints/Weather_BP.Humidity` newSnowDensity _bp_weather))

(fn `UserConstructionScript`
  ;[1 1 1] 获取天气蓝图actor和天空球actor
  (bind _returnvalue (`GameplayStatics.GetActorOfClass` "/Game/UltraDynamicSky/Blueprints/Ultra_Dynamic_Sky_BP.Ultra_Dynamic_Sky_BP_C"))
  (set `self.ultra_dynamic_sky_sphere` _returnvalue)
  (bind _returnvalue_2 (`GameplayStatics.GetActorOfClass` "/Game/Dynamic_Weather/Blueprints/Weather_BP.Weather_BP_C"))
  (set `self.BP_Weather` _returnvalue_2)
  (bind _returnvalue_3 (`GameplayStatics.GetActorOfClass` "/Script/Engine.SkyLight"))
  (set `self.sky_light` _returnvalue_3)
  (bind _returnvalue_4 (`GameplayStatics.GetActorOfClass` "/Script/Engine.ExponentialHeightFog"))
  (set `self.EXP_fog` _returnvalue_4))