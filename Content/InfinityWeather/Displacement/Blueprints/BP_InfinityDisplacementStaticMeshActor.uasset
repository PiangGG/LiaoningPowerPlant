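; Static mesh actor that supplies a displacement shape to the Infinity Weather displacement system.
; On construction and BeginPlay it caches itself, shape type and shape transform, and flags itself dynamic if its mesh is Movable.
; AddDisplacementShapeData appends that cached data to the given stack, refreshing the transform only for movable actors to spare static ones the recomputation.
; GetDisplacementTexture is left empty.
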(event `self.ReceiveBeginPlay`
  (`self.SaveSelf`))

(fn `AddDisplacementShapeData`
  (params (Stack :type "Array of /Game/InfinityWeather/Displacement/Blueprints/BS_DisplacementShape Structure (by ref)"))
  (returns (Added :type Boolean))
  (if (`self.IsDynamic`)
    (bind _structout (setmembers `/Game/InfinityWeather/Displacement/Blueprints/BS_DisplacementShape` :`StructRef` (`self.StaticShapeData`) :`Transform` (`self.GetShapeTransform`)))
    (`KismetArrayLibrary.Array_Add` Stack _structout)
    (return true)
    (else
      (`KismetArrayLibrary.Array_Add` Stack (`self.StaticShapeData`))
      (return true))))

(fn `GetDisplacementTexture`
  (returns (Texture :type "Texture2D Object Reference"))
  (return null))

(fn `SaveSelf`
  (bind (_shapedata_actor _shapedata_type) (break `/Game/InfinityWeather/Displacement/Blueprints/BS_DisplacementShape` (`self.ShapeData`)))
  (set `self.StaticShapeData` (make `/Game/InfinityWeather/Displacement/Blueprints/BS_DisplacementShape` self _shapedata_type (`self.GetShapeTransform`)))
  (set `self.IsDynamic` (`|EnumEquality` (`SceneComponent.Mobility` (`self.StaticMeshComponent`)) "Movable")))

(fn `UserConstructionScript`
  (`self.SaveSelf`))